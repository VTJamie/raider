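; Behavior tree decorator that checks whether the AI's target is within range of its selected ability.
; It reads the ability and target from blackboard keys, casts them to BP_TargetAbility_C and BP_Character_Base, then asks the ability's ActorWithinRange.
; The result is stored in WithinRange, which is returned unchanged when the ability cast fails or the target is invalid.
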(fn `PerformConditionCheckAI`
  (params (OwnerController :type "AIController Object Reference") (ControlledPawn :type "Pawn Object Reference"))
  (returns (ReturnValue :type Boolean))
  (locals (`Within Range` :type Boolean))
  (bind _returnvalue (`BTFunctionLibrary.GetBlackboardValueAsActor` (`self.BB Target`)))
  (bind _asbp_target_ability_c (cast `/Game/Shared/Ability/BP_TargetAbility_C` (`BTFunctionLibrary.GetBlackboardValueAsObject` (`self.BB Ability`)))
    (:`then`
      (`/Engine/EditorBlueprintResources/StandardMacros.IsValid` _returnvalue
        (:`Is Valid`
          (bind _asbp_character_base (cast `/Game/Player/BP_Character_Base` _returnvalue))
          (bind _within_range (`/Game/Shared/Ability/BP_TargetAbility_I.Actor Within Range` _asbp_target_ability_c _asbp_character_base))
          (set `local.Within Range` _within_range))
        (:`Is Not Valid`
          _)))
    (:`CastFailed`
      _))
  (return (`local.Within Range`)))