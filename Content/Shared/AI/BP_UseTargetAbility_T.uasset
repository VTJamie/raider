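; Behavior tree task that makes an AI use a target ability on a target, both read from the blackboard.
; On execute it checks the target actor is valid, casts the blackboard ability to BP_TargetAbility, calls UseAbilityOnTarget and finishes with success.
; An invalid target or ability finishes with failure.
; A target that is not a BP_Character_Base stops execution without finishing the task.
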(event `self.ReceiveExecuteAI`
  (params (OwnerController :type "AIController Object Reference") (ControlledPawn :type "Pawn Object Reference"))
  (bind _returnvalue (`BTFunctionLibrary.GetBlackboardValueAsActor` (`self.BB Target`)))
  (if (`KismetSystemLibrary.IsValid` _returnvalue)
    (bind _asbp_target_ability_c (cast `/Game/Shared/Ability/BP_TargetAbility_C` (`BTFunctionLibrary.GetBlackboardValueAsObject` (`self.BB Ability`)))
      (:`then`
        (bind _asbp_character_base (cast `/Game/Player/BP_Character_Base` _returnvalue))
        (`/Game/Shared/Ability/BP_TargetAbility_C.Use Ability On Target` _asbp_target_ability_c _asbp_character_base)
        (`self.FinishExecute` true))
      (:`CastFailed`
        (`self.FinishExecute` false :!label _label)))
    (else
      (goto _label))))