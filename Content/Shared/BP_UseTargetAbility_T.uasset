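; Behavior Tree task that makes the controlled pawn use a target ability on the actor stored in a Blackboard key.
; It looks up the pawn's component of the configured ability class, casts it to BP_TargetAbility and calls UseAbilityOnTarget, then finishes successfully.
; An invalid target fails the task.
; A failed cast only prints the component's name and never finishes execution.
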(event `self.ReceiveExecuteAI`
  (params (OwnerController :type "AIController Object Reference") (ControlledPawn :type "Pawn Object Reference"))
  (bind _returnvalue (`Actor.GetComponentByClass` ControlledPawn (`self.Ability To Use`)))
  (bind _returnvalue_2 (`BTFunctionLibrary.GetBlackboardValueAsActor` (`self.BB Target`)))
  (if (`KismetSystemLibrary.IsValid` _returnvalue_2)
    (bind _asbp_target_ability_c (cast `/Game/Shared/BP_TargetAbility_C` _returnvalue)
      (:`then`
        (`/Game/Shared/BP_TargetAbility_C.Use Ability On Target` _asbp_target_ability_c _returnvalue_2)
        (`self.FinishExecute` true))
      (:`CastFailed`
        (`KismetSystemLibrary.PrintString` (`KismetSystemLibrary.GetDisplayName` _returnvalue))))
    (else
      (`self.FinishExecute` false))))