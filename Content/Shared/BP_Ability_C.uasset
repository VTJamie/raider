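; BP_Ability is a base ability attached to an owning actor, providing cooldown and range checks.
; Executing the ability starts a one-shot timer for the cooldown, whose expiry clears and resets the stored handle.
; Readiness is derived from that timer's remaining time, which reads zero when no valid handle exists.
; The range check compares a location's distance from the owner against the ability range.
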(event `Executed Ability`
  (bind _returnvalue (`KismetSystemLibrary.K2_SetTimerDelegate` (delegate `self.Reset Ability Timer`) (`self.Cooldown`)))
  (set `self.Current Timer` _returnvalue))

(event `self.Reset Ability Timer`
  (if (`KismetSystemLibrary.K2_IsValidTimerHandle` (`self.Current Timer`))
    (`KismetSystemLibrary.K2_ClearAndInvalidateTimerHandle` (`self.Current Timer`)))
  (set `self.Current Timer` (struct)))

(fn `Ability Is Ready`
  (returns (`Is Ready` :type Boolean))
  (bind _remaining_time (`self.Remaining Time`))
  (return (<= _remaining_time 0.0)))

(fn `Remaining Time`
  (returns (`Remaining Time` :type "Float (double-precision)"))
  (locals (`Return Remaining Time` :type "Float (double-precision)"))
  (bind _current_timer (`self.Current Timer`))
  (if (`KismetSystemLibrary.K2_IsValidTimerHandle` _current_timer)
    (set `local.Return Remaining Time` (`KismetSystemLibrary.K2_GetTimerRemainingTimeHandle` _current_timer))
    (else
      (set `local.Return Remaining Time` 0.0)))
  (return (`local.Return Remaining Time`)))

(fn `Within Range`
  (params (Location :type "Vector Structure"))
  (returns (`Is In Range` :type Boolean))
  (return (<= (`KismetMathLibrary.Vector_Distance` Location (`Actor.K2_GetActorLocation` (`self.GetOwner`))) (`self.Ability Range`))))