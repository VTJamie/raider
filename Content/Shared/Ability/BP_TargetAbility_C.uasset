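; Base Blueprint for character abilities that are used on a target actor.
; UseAbilityonTarget runs the ability only when the target's location is within range, the ability is ready and the owner is a Character.
; It then calls HandleAbilityOnTarget with the target and owner, followed by ExecutedAbility.
; Range, readiness and effect logic come from functions defined outside this graph.
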(event `self.Use Ability On Target`
  (params (Target :type "Actor Object Reference"))
  (bind _within_range (`self.Actor Within Range` Target))
  (if _within_range
    (bind _is_ready (`/Game/Shared/Ability/BP_Ability_I.Ability Is Ready`))
    (if _is_ready
      (bind _ascharacter (cast `Character` (`self.GetOwner`)))
      (`self.Handle Ability On Target` Target _ascharacter)
      (`self.Executed Ability`))))

(fn `Actor Within Range`
  (params (Target :type "Actor Object Reference"))
  (returns (`Within Range` :type Boolean))
  (bind _is_in_range (`self.Within Range` (`Actor.K2_GetActorLocation` Target)))
  (return _is_in_range))