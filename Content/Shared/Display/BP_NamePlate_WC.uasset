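; BP_NamePlate_WC is a widget component that shows a name plate and health bar for its owning actor through BP_InfoPanel_W.
; On BeginPlay it sets the name text to the owner's display name.
; Each Tick it polls the health percentage from the BP_Character_Base owner's Stats to update the bar, then rotates to face the first player's camera.
; Non-character owners get neither health updates nor rotation, as the failed cast stops Tick.
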(event `self.ReceiveBeginPlay`
  (bind _asbp_info_panel_w (cast `/Game/Shared/Display/BP_InfoPanel_W` (`self.GetUserWidgetObject`)))
  (`TextBlock.SetText` (`/Game/Shared/Display/BP_InfoPanel_W.NamePlate` _asbp_info_panel_w) (`KismetTextLibrary.Conv_StringToText` (`KismetSystemLibrary.GetDisplayName` (`self.GetOwner`)))))

(event `self.ReceiveTick`
  (params (DeltaSeconds :type "Float (single-precision)"))
  (bind _asbp_info_panel_w (cast `/Game/Shared/Display/BP_InfoPanel_W` (`self.GetUserWidgetObject`)))
  (bind _asbp_character_base (cast `/Game/Player/BP_Character_Base` (`self.GetOwner`)))
  (bind _health_percentage (`/Game/Shared/BP_Stats_I.Get Health Percentage` (`/Game/Player/BP_Character_Base.Stats` _asbp_character_base)))
  (`ProgressBar.SetPercent` (`/Game/Shared/Display/BP_InfoPanel_W.HealthBar` _asbp_info_panel_w) _health_percentage)
  (`self.K2_SetWorldRotation` (`KismetMathLibrary.FindLookAtRotation` (`self.K2_GetComponentLocation`) (`PlayerCameraManager.GetCameraLocation` (`GameplayStatics.GetPlayerCameraManager` 0)))))