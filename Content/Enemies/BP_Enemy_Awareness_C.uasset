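; BP_Enemy_Awareness_C fills an enemy's view of who is friend or foe in the level when play begins.
; Every BP_Player_Base actor is stored by display name in the LevelContent Enemies map and given a fixed starting threat level.
; Inside that same player loop, all BP_Enemy_Base actor names are added to Allies with no value wired, so that pass repeats per player.
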(event `self.ReceiveBeginPlay`
  (bind (_enemies _allies _threatlevels) (break `/Game/Shared/S_Awareness` (`self.Level Content`)))
  (bind _outactors (`GameplayStatics.GetAllActorsOfClass` "/Game/Player/BP_Player_Base.BP_Player_Base_C"))
  (for _array_element _outactors
    (bind _returnvalue (`KismetSystemLibrary.GetDisplayName` _array_element))
    (`BlueprintMapLibrary.Map_Add` _enemies _returnvalue _array_element)
    (`BlueprintMapLibrary.Map_Add` _threatlevels _returnvalue 10)
    (bind _outactors_2 (`GameplayStatics.GetAllActorsOfClass` "/Game/Enemies/BP_Enemy_Base.BP_Enemy_Base_C"))
    (for _array_element_2 _outactors_2
      (`BlueprintMapLibrary.Map_Add` (`.Allies_17_FFE93BE581450FCC37A3CBA633571D8D` (break `/Game/Shared/S_Awareness` (`self.Level Content`))) (`KismetSystemLibrary.GetDisplayName` _array_element_2)))))