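; BP_ky_shot_fire is a fire projectile actor from AdvancedMagicFX12 that flies forward and reacts to enemies.
; A timeline started on BeginPlay moves the FX component along relative X, scaled by ShotSpeed, the curve and delta time.
; Chained delays from the timeline update deactivate the FX and Sphere collision, then destroy the actor.
; Overlapping a BP_Enemy_Base spawns a fire hit emitter and destroys it immediately, with no damage applied here.
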(event `self.ReceiveBeginPlay`
  (bind (_direction _newtrack_0) (`Timeline|Timeline_0` :!via `PlayFromStart`)
    (:`Update`
      (`SceneComponent.K2_AddRelativeLocation` (`self.FX`) (`KismetMathLibrary.MakeVector` (* (* (`self.shotSpeed`) _newtrack_0) (stale `self.ReceiveTick` DeltaSeconds))) false false)
      (`KismetSystemLibrary.Delay` 1.5)
      (`ActorComponent.Deactivate` (`self.FX`))
      (`PrimitiveComponent.SetCollisionEnabled` (`self.Sphere`) "NoCollision")
      (`KismetSystemLibrary.Delay` 0.5)
      (`self.K2_DestroyActor`))))

(event `self.ReceiveTick`
  (params (DeltaSeconds :type "Float (single-precision)")))

(event `self.ReceiveActorBeginOverlap`
  (params (OtherActor :type "Actor Object Reference"))
  (cast `/Game/Enemies/BP_Enemy_Base` OtherActor)
  (`GameplayStatics.SpawnEmitterAtLocation` "/Game/AdvancedMagicFX12/Particles/P_ky_hit_fire.P_ky_hit_fire" (`SceneComponent.K2_GetComponentLocation` (`self.FX`)))
  (`self.K2_DestroyActor`))

(fn `UserConstructionScript`)