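; Character stats Blueprint that holds attributes (Strength, Intelligence, Wisdom, Fortitude, Dexterity) and manages Health.
; BeginPlay resets each attribute to its base and derives Health from Fortitude.
; Healing clamps to max and returns the amount gained, alongside health percentage and death queries.
; TakeDamage subtracts unmitigated damage, ignoring Type, and calls Died at zero or below, returning amounts only on that branch.
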(event `self.ReceiveBeginPlay`
  (bind _dexterity (`self.Dexterity`))
  (bind _strength (`self.Strength`))
  (bind _intelligence (`self.Intelligence`))
  (bind _wisdom (`self.Wisdom`))
  (bind _fortitude (`self.Fortitude`))
  (bind (_current _base) (break `/Game/Player/S_Stat` _dexterity))
  (bind (_current_2 _base_2) (break `/Game/Player/S_Stat` _strength))
  (bind (_current_3 _base_3) (break `/Game/Player/S_Stat` _intelligence))
  (bind (_current_4 _base_4) (break `/Game/Player/S_Stat` _wisdom))
  (bind (_current_5 _base_5) (break `/Game/Player/S_Stat` _fortitude))
  (bind _returnvalue (* (`.Current_2_2889A172CB46CD8D2F6578972377782C` (break `/Game/Player/S_Stat` (`self.Fortitude`))) 100))
  (setmembers `/Game/Player/S_Stat` :`StructRef` _strength :`Current` _base_2 :`Max` _base_2)
  (setmembers `/Game/Player/S_Stat` :`StructRef` _intelligence :`Current` _base_3 :`Max` _base_3)
  (setmembers `/Game/Player/S_Stat` :`StructRef` _wisdom :`Current` _base_4 :`Max` _base_4)
  (setmembers `/Game/Player/S_Stat` :`StructRef` _fortitude :`Current` _base_5 :`Max` _base_5)
  (setmembers `/Game/Player/S_Stat` :`StructRef` _dexterity :`Current` _base :`Max` _base)
  (setmembers `/Game/Player/S_Stat` :`StructRef` (`self.Health`) :`Current` _returnvalue :`Base` _returnvalue :`Max` _returnvalue))

(fn `Get Healed`
  (params (Amount :type Integer))
  (returns (`Actual Amount` :type Integer))
  (locals (`Starting Health` :type Integer))
  (bind _health (`self.Health`))
  (bind (_current _base _max) (break `/Game/Player/S_Stat` _health))
  (set `local.Starting Health` _current)
  (bind _structout (setmembers `/Game/Player/S_Stat` :`StructRef` _health :`Current` (`KismetMathLibrary.Min` _max (+ Amount _current))))
  (return (- (`.Current_2_2889A172CB46CD8D2F6578972377782C` (break `/Game/Player/S_Stat` _structout)) (`local.Starting Health`))))

(fn `Get Health Percentage`
  (returns (`Health Percentage` :type "Float (double-precision)"))
  (bind (_current _base _max) (break `/Game/Player/S_Stat` (`self.Health`)))
  (return (/ (`KismetMathLibrary.Conv_IntToDouble` _current) (`KismetMathLibrary.Conv_IntToDouble` _max))))

(fn `Is Dead`
  (returns (`Is Dead` :type Boolean))
  (return (<= (`.Current_2_2889A172CB46CD8D2F6578972377782C` (break `/Game/Player/S_Stat` (`self.Health`))) 0)))

(fn `Take Damage`
  (params (Type :type "/Game/Shared/E_DamageType Enum" :default "NewEnumerator0") (Amount :type Integer))
  (returns (`Actual Amount` :type Integer) (`Mitigated Amount` :type Integer))
  (bind _health (`self.Health`))
  (bind _structout (setmembers `/Game/Player/S_Stat` :`StructRef` _health :`Current` (- (`.Current_2_2889A172CB46CD8D2F6578972377782C` (break `/Game/Player/S_Stat` _health)) Amount)))
  (if (<= (`.Current_2_2889A172CB46CD8D2F6578972377782C` (break `/Game/Player/S_Stat` _structout)) 0)
    (`self.Died`)
    (return Amount 0)))