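; BP_Player_Awareness builds a registry of the player and enemy actors present in the level when play begins.
; On BeginPlay it finds all BP_Player_Base actors and adds them to LevelContents.Allies, keyed by display name.
; The BP_Enemy_Base search that fills LevelContents.Enemies is nested inside the ally loop, so it repeats for each ally and only runs when one exists.
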(event `self.ReceiveBeginPlay`
  (bind _outactors (`GameplayStatics.GetAllActorsOfClass` "/Game/Player/BP_Player_Base.BP_Player_Base_C"))
  (for _array_element _outactors
    (`BlueprintMapLibrary.Map_Add` (`.Allies_17_FFE93BE581450FCC37A3CBA633571D8D` (break `/Game/Shared/S_Awareness` (`self.LevelContents`))) (`KismetSystemLibrary.GetDisplayName` _array_element) _array_element)
    (bind _outactors_2 (`GameplayStatics.GetAllActorsOfClass` "/Game/Enemies/BP_Enemy_Base.BP_Enemy_Base_C"))
    (for _array_element_2 _outactors_2
      (`BlueprintMapLibrary.Map_Add` (`.Enemies_16_26CA4983D3438EEC79013F8E9046FBE0` (break `/Game/Shared/S_Awareness` (`self.LevelContents`))) (`KismetSystemLibrary.GetDisplayName` _array_element_2) _array_element_2))))